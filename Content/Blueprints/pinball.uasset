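; Pinball is a weapon actor that assigns itself as the Weapon of any MyCharacter that overlaps it.
; Its pinball event takes a toggle that enables or stops automatic fire, run as a self-repeating loop gated by a short delay and a FireDelay flag.
; Each shot spawns a Bullet at the transform of player character 0, not at the weapon's own transform.
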(event Custom|pinball
  (params (toggle :type Boolean))
  (bind _output_get (Variables|Default|Setcan%20fire toggle))
  (if _output_get
    (if (and (Variables|Default|Getcan%20fire) (not (Variables|Default|Getfire%20delay))) :!label _label
      (Variables|Default|Setfire%20delay true)
      (CallFunction|SpawnProjectile)
      (Utilities|FlowControl|Delay 0.2)
      (Variables|Default|Setfire%20delay false)
      (goto _label))))

(event EventBeginPlay)

(event Collision|EventActorBeginOverlap
  (params (OtherActor :type Actor%20Object%20Reference))
  (bind _asmy_character (Utilities|Casting|CastToMyCharacter OtherActor))
  (Variables|/Game/Character/MyCharacter.MyCharacter_C|Setweapon _asmy_character self))

(event EventTick
  (params (DeltaSeconds :type Float%20%28single-precision%29)))

(fn ConstructionScript)

(fn SpawnProjectile
  (Game|SpawnActorfromClass "/Game/Blueprints/bullet.bullet_C" (Transformation|GetActorTransform (Game|GetPlayerCharacter 0)) "Undefined" 0 0))